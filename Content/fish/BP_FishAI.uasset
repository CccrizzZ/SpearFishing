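; Swimming fish AI that wanders through a water volume and can be killed by a spear.
; Tick eases rotation toward a random heading and applies movement input, re-rolling every few seconds via Delay, or reversing horizontally inside the stranded TriggerCapsule.
; Living fish outside both the first-found PhysicsVolume and that capsule are destroyed.
; A simulating "spear_body" hit attaches the spear, enables physics and swaps to a dead material, with gravity toggled by water position.
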(event EventBeginPlay
  (Pawn|Components|CharacterMovement|SetMovementMode (Variables|Character|GetCharacterMovement) "MOVE_Swimming" 0)
  (CallFunction|SetRandomMoveDirection (Math|Random|RandomIntegerinRange 0 2)))

(event Collision|EventActorBeginOverlap
  (params (OtherActor :type Actor%20Object%20Reference)))

(event EventTick
  (params (DeltaSeconds :type Float%20%28single-precision%29))
  (bind _sphere (Variables|Default|GetSphere))
  (if (Variables|Default|GetisDead)
    (Rendering|SetVisibility (Variables|Collision|GetCapsuleComponent) false false)
    (bind _isinvolume (CallFunction|IsinPhysicsVolume))
    (if (and _isinvolume (< (.z (Transformation|GetWorldLocation (Variables|Default|GetSphere))) 0.0))
      (Physics|SetEnableGravity _sphere false)
      (else
        (Physics|SetEnableGravity _sphere true)))
    (else
      ;[0.5 1 0] If fish is out of bound, kill it
      (bind _isinvolume_2 (CallFunction|IsinPhysicsVolume))
      (if _isinvolume_2
        ;[0.5937 1 0] LerpRotateFish
        (Transformation|SetActorRotation (Math|Rotator|Lerp(Rotator) (Transformation|GetActorRotation) (Math|Conversions|RotationFromXVector (Variables|Default|GetMoveDirection)) DeltaSeconds) :!label _label)
        ;[0.6641 0 1] Move the fish
        (Pawn|Input|AddMovementInput (Variables|Default|GetMoveDirection) (Math|Random|RandomFloatinRange 1.0 5.0) false)
        (if (Variables|Default|GetReversed)
          (Utilities|FlowControl|Delay 3.0)
          (Variables|Default|SetReversed false)
          (else
            (Utilities|FlowControl|Delay 3.0)
            (CallFunction|SetRandomMoveDirection 1)))
        (else
          (bind _isinstranded (CallFunction|IsinStrandedZone))
          (if _isinstranded
            (goto _label)
            (else
              (Actor|DestroyActor)
              (Development|PrintString "FishKilled"))))))))

(event Collision|EventHit
  (params (MyComp :type Primitive%20Component%20Object%20Reference) (Other :type Actor%20Object%20Reference) (OtherComp :type Primitive%20Component%20Object%20Reference) (bSelfMoved :type Boolean) (HitLocation :type Vector :default "0, 0, 0") (HitNormal :type Vector :default "0, 0, 0") (NormalImpulse :type Vector :default "0, 0, 0") (Hit :type Hit%20Result%20Structure%20%28by%20ref%29))
  (bind _sphere (Variables|Default|GetSphere))
  (if (and (Physics|IsSimulatingPhysics OtherComp "None") (Utilities|Enum|Equal(Enum) (Utilities|GetObjectName OtherComp) "spear_body"))
    (Transformation|AttachComponentToComponent OtherComp (Variables|Default|GetSphere) "None" "KeepWorld" "KeepWorld" "KeepWorld" true)
    (Physics|SetSimulatePhysics _sphere true)
    (Rendering|Material|SetMaterial _sphere 0 "/Game/fish/M_fish_dead.M_fish_dead")
    (Variables|Default|SetisDead true)))

(fn ConstructionScript)

(fn SetRandomMoveDirection
  (params (UpMiddleDown :type Integer))
  ;[0 1 0.3906] Reverse fish x y movement if collided with stranded trigger
  (bind _outactors (Actor|GetAllActorsOfClass "/Script/Engine.TriggerCapsule"))
  (if (Collision|IsOverlappingActor (Variables|Collision|GetCapsuleComponent) (Utilities|Array|Get(acopy) _outactors) :!class /Script/Engine.PrimitiveComponent)
    (CallFunction|ReverseMovingDirection)
    (else
      (switch int UpMiddleDown
        (:0
          ;[1 0.3281 0] Down
          (Variables|Default|SetMoveDirection (Math|Vector|MakeVector (Math|Random|RandomFloatinRange -1.0 1.0) (Math|Random|RandomFloatinRange -1.0 1.0) (Math|Random|RandomFloatinRange -1.0 0.0))))
        (:1
          ;[1 0.3281 0] Middle
          (Variables|Default|SetMoveDirection (Math|Vector|MakeVector (Math|Random|RandomFloatinRange -1.0 1.0) (Math|Random|RandomFloatinRange -1.0 1.0) (Math|Random|RandomFloatinRange -0.2 0.2))))
        (:2
          ;[1 0.3281 0] Up
          (Variables|Default|SetMoveDirection (Math|Vector|MakeVector (Math|Random|RandomFloatinRange -1.0 1.0) (Math|Random|RandomFloatinRange -1.0 1.0) (Math|Random|RandomFloatinRange 0.0 1.0))))))))

(fn ReverseMovingDirection
  (Variables|Default|SetMoveDirection (Math|Vector|MakeVector (.x (* (Variables|Default|GetMoveDirection) -1.0)) (.y (* (Variables|Default|GetMoveDirection) -1.0)) 0.0))
  (Variables|Default|SetReversed true))

(fn IsinPhysicsVolume
  (bind _outactors (Actor|GetAllActorsOfClass "/Script/Engine.PhysicsVolume"))
  (return (Collision|IsOverlappingActor (Utilities|Array|Get(acopy) _outactors) self :!class /Script/Engine.Actor)))

(fn IsinStrandedZone
  (bind _outactors (Actor|GetAllActorsOfClass "/Script/Engine.TriggerCapsule"))
  (return (Collision|IsOverlappingActor (Utilities|Array|Get(acopy) _outactors) self :!class /Script/Engine.Actor)))