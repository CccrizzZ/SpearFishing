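; BP_SpearGun is the spear gun actor, with an indicator screen and distance readout driven by externally callable events.
; SetRed and SetGreen swap the screen between hit and caught-fish materials, hiding the readout for red and showing it for green.
; SetIndicatorText subtracts a one-meter offset from the supplied distance and displays it in rounded meters.
; It contains no firing or detection logic, and Tick is empty.
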(event Custom|SetRed
  (Rendering|Material|SetMaterial (Variables|Default|GetIndicatorScreen) 0 "/Game/SpearGun/M_HitMaterial.M_HitMaterial")
  (Rendering|SetVisibility (Variables|Default|GetDistanceIndicator) false false))

(event Custom|SetGreen
  (Rendering|Material|SetMaterial (Variables|Default|GetIndicatorScreen) 0 "/Game/SpearGun/M_CaughtFIsh.M_CaughtFish")
  (Rendering|SetVisibility (Variables|Default|GetDistanceIndicator) true false))

(event Custom|SetIndicatorText
  (params (Distance :type Float%20%28single-precision%29))
  (Rendering|Components|TextRender|SetText (Variables|Default|GetDistanceIndicator) (Utilities|Text|ToText(String) (Utilities|String|Append (Utilities|String|ToString(Integer) (Math|Float|Round (/ (- Distance 1e+02) 1e+02))) "m"))))

(event EventBeginPlay)

(event Collision|EventActorBeginOverlap
  (params (OtherActor :type Actor%20Object%20Reference)))

(event EventTick
  (params (DeltaSeconds :type Float%20%28single-precision%29)))

(fn ConstructionScript)