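; Spear projectile actor that reacts to striking a physics-simulating component named "TestTarget".
; On such a hit it swaps the component to a hit material, applies an impulse scaled from the spear's velocity at the spear's location, then destroys itself.
; ToggleSimulatingPhysics switches physics on the Spear component.
; The timed self-destroy is unconnected, so spears that miss are not cleaned up here.
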(event EventBeginPlay)

(event Collision|EventActorBeginOverlap
  (params (OtherActor :type Actor%20Object%20Reference)))

(event EventTick
  (params (DeltaSeconds :type Float%20%28single-precision%29)))

(event Collision|EventHit
  (params (MyComp :type Primitive%20Component%20Object%20Reference) (Other :type Actor%20Object%20Reference) (OtherComp :type Primitive%20Component%20Object%20Reference) (bSelfMoved :type Boolean) (HitLocation :type Vector :default "0, 0, 0") (HitNormal :type Vector :default "0, 0, 0") (NormalImpulse :type Vector :default "0, 0, 0") (Hit :type Hit%20Result%20Structure%20%28by%20ref%29))
  (if (and (Physics|IsSimulatingPhysics OtherComp "None") (Utilities|Enum|Equal(Enum) (Utilities|GetObjectName OtherComp) "TestTarget"))
    (Rendering|Material|SetMaterial OtherComp 0 "/Game/SpearGun/M_HitMaterial.M_HitMaterial")
    (Physics|AddImpulseatLocation OtherComp (* (Transformation|GetVelocity) 5e+03) (Transformation|GetActorLocation) "None")
    (Actor|DestroyActor)))

(fn ConstructionScript)

(fn ToggleSimulatingPhysics
  (params (isSimulating :type Boolean))
  (Physics|SetSimulatePhysics (Variables|Default|Getspear) isSimulating))